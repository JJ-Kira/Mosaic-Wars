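; BP_Platform is a square tiled platform actor for Mosaic Wars, with its size driven by PlatformSize.
; The construction script runs a nested loop that adds instances to the Tiles component in local space, forming a flat, evenly spaced grid from the actor's origin.
; The event graph holds only disabled placeholder events, so the actor has no runtime logic of its own.
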(fn `UserConstructionScript`
  (bind _platformsize (`self.PlatformSize`))
  (for _index (range (+ _platformsize 1))
    (for _index_2 (range (+ _platformsize 1))
      (`InstancedStaticMeshComponent.AddInstance` (`self.Tiles`) (`KismetMathLibrary.MakeTransform` (`KismetMathLibrary.MakeVector` (`KismetMathLibrary.Conv_IntToDouble` (* _index 100)) (`KismetMathLibrary.Conv_IntToDouble` (* _index_2 100)))) false))))