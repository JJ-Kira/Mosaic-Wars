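; Menu player controller for MosaicWars that handles the front-end UI and session exit.
; On BeginPlay the local controller shows the mouse cursor and switches to UI-only input.
; CreateLobbyMenu creates the WB_LobbyMenu widget once, caches it and adds it to the viewport.
; EndClientSession destroys the session, then opens the MainMenu level on the completion callback's immediate exec pin.
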(event `self.ReceiveBeginPlay`
  (if (`self.IsLocalController`)
    (set `self.bShowMouseCursor` true)
    (`WidgetBlueprintLibrary.SetInputMode_UIOnlyEx` self null)))

(event `EndClientSession`
  (`DestroySessionCallbackProxy.DestroySession` self
    (:`then`
      (`GameplayStatics.OpenLevel` "MainMenu"))))

(event `CreateLobbyMenu`
  (`self.UI_ShowLobbyMenu`))

(fn `UI_ShowLobbyMenu`
  (`/Engine/EditorBlueprintResources/StandardMacros.IsValid` (`self.LobbyMenu`)
    (:`Is Valid`
      _)
    (:`Is Not Valid`
      (bind _returnvalue (`|CreateWidget` "/Game/MosaicWars/Widgets/WB_LobbyMenu.WB_LobbyMenu_C" self))
      (set `self.LobbyMenu` _returnvalue)))
  (`UserWidget.AddToViewport` (`self.LobbyMenu`) 0))

(fn `UserConstructionScript`)