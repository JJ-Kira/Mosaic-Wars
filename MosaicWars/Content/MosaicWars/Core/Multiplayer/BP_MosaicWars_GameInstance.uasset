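; Game instance for Mosaic Wars that shows the main menu and persists the player's profile.
; Showing the menu creates or reuses the WB_MainMenu widget, switches to UI-only input with a visible cursor, then fills the name field from the profile.
; The profile is loaded from an SG_PlayerProfile save slot, or saved fresh if none exists.
; Changing the player name rebuilds the profile struct and saves it immediately.
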(event `ChangePlayerName`
  (params (NewPlayerName :type Text))
  (set `self.PlayerProfile_Info` (make `/Game/MosaicWars/Core/SaveData/S_PlayerProfile` NewPlayerName))
  (`self.SaveProfile`))

(fn `CheckForSave`
  (bind _returnvalue (`GameplayStatics.DoesSaveGameExist` (`self.PlayerProfile_Slot`)))
  (if _returnvalue
    (`self.LoadProfile`)
    (else
      (`self.SaveProfile`)))
  (return))

(fn `LoadProfile`
  (bind _returnvalue (`GameplayStatics.LoadGameFromSlot` (`self.PlayerProfile_Slot`)))
  (bind _assg_player_profile (cast `/Game/MosaicWars/Core/SaveData/SG_PlayerProfile` _returnvalue))
  (set `self.PlayerProfile_Info` (`/Game/MosaicWars/Core/SaveData/SG_PlayerProfile.PlayerProfile` _assg_player_profile))
  (return))

(fn `SaveProfile`
  (`/Engine/EditorBlueprintResources/StandardMacros.IsValid` (`self.PlayerProfile`)
    (:`Is Valid`
      _)
    (:`Is Not Valid`
      (bind _returnvalue (`GameplayStatics.CreateSaveGameObject` "/Game/MosaicWars/Core/SaveData/SG_PlayerProfile.SG_PlayerProfile_C"))
      (set `self.PlayerProfile` _returnvalue)))
  (set `/Game/MosaicWars/Core/SaveData/SG_PlayerProfile.PlayerProfile` (`self.PlayerProfile_Info`) (`self.PlayerProfile`))
  (`GameplayStatics.SaveGameToSlot` (`self.PlayerProfile`) (`self.PlayerProfile_Slot`)))

(fn `UI_ShowMainMenu`
  (bind _returnvalue (`GameplayStatics.GetPlayerController` 0))
  (`/Engine/EditorBlueprintResources/StandardMacros.IsValid` (`self.MainMenu_WB`)
    (:`Is Valid`
      _)
    (:`Is Not Valid`
      (bind _returnvalue_2 (`|CreateWidget` "/Game/MosaicWars/Widgets/WB_MainMenu.WB_MainMenu_C" (`GameplayStatics.GetPlayerController` 0)))
      (set `self.MainMenu_WB` _returnvalue_2)))
  (`UserWidget.AddToViewport` (`self.MainMenu_WB`) 0)
  (`WidgetBlueprintLibrary.SetInputMode_UIOnlyEx` _returnvalue null)
  (set `PlayerController.bShowMouseCursor` true _returnvalue)
  (`self.CheckForSave`)
  (`EditableText.SetText` (`/Game/MosaicWars/Widgets/WB_MainMenu.Input_Name` (`self.MainMenu_WB`)) (`.PlayerName_2_6FC52DD14023C744D6DA548A7FD1CCBC` (break `/Game/MosaicWars/Core/SaveData/S_PlayerProfile` (`self.PlayerProfile_Info`))))
  (return))