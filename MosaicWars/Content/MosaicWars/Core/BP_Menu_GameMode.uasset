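; Menu game mode for Mosaic Wars that manages the multiplayer lobby's player roster and readiness.
; In the Lobby level, each new player is registered, given lobby UI and mouse input, and spawned at a PlayerStart named by join index.
; Parallel arrays track controllers, profiles and ready flags.
; Ready toggles and logouts trigger UpdateLobby, which copies profiles to PlayerStates and pushes names and readiness to controllers.
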(event `self.HandleStartingNewPlayer`
  (params (NewPlayer :type "PlayerController Object Reference"))
  ;[1 1 1] Set up lobby UI & spawn player
  (bind _returnvalue (`GameplayStatics.GetCurrentLevelName` true))
  (switch `string` _returnvalue
    (:`Lobby`
      (bind _asbp_menu_controller (cast `/Game/MosaicWars/Core/Menu/BP_MenuController` NewPlayer))
      (bind _returnvalue_2 (`KismetArrayLibrary.Array_Add` (`self.ConnectedPlayers`) _asbp_menu_controller))
      (`KismetArrayLibrary.Array_Set` (`self.bIsPlayerReady`) _returnvalue_2 false true)
      (`/Game/MosaicWars/Core/Menu/BP_MenuController.CreateLobbyMenu` _asbp_menu_controller)
      (`/Game/MosaicWars/Core/Menu/BP_MenuController.CreateLobbyMenu` _asbp_menu_controller)
      (`/Game/MosaicWars/Core/Menu/BP_MenuController.InitialLobbySetup` _asbp_menu_controller)
      (`self.RestartPlayerAtPlayerStart` NewPlayer (`self.K2_FindPlayerStart` NewPlayer (`KismetStringLibrary.Conv_IntToString` _returnvalue_2)))
      (`WidgetBlueprintLibrary.SetInputMode_GameAndUIEx` NewPlayer null "LockAlways")
      (set `PlayerController.bShowMouseCursor` true NewPlayer))))

(event `UpdateLobby`
  ;[1 1 1] Update Player Name and Readiness List in the Lobby
  (`KismetArrayLibrary.Array_Clear` (`self.PlayerProfiles`))
  (for (_array_element _array_index) (`self.ConnectedPlayers`)
    (bind _localplayerprofile (`/Game/MosaicWars/Core/Menu/BP_MenuController.LocalPlayerProfile` _array_element))
    (`KismetArrayLibrary.Array_Set` (`self.PlayerProfiles`) _array_index _localplayerprofile true)
    (bind _asbp_mosaic_wars_player_state (cast `/Game/MosaicWars/Core/Multiplayer/BP_MosaicWars_PlayerState` (`Controller.PlayerState` _array_element)))
    (set `/Game/MosaicWars/Core/Multiplayer/BP_MosaicWars_PlayerState.PlayerProfile` _localplayerprofile _asbp_mosaic_wars_player_state))
  (for _array_element_2 (`self.ConnectedPlayers`)
    (`/Game/MosaicWars/Core/Menu/BP_MenuController.UpdatePlayerNames` _array_element_2 (`self.PlayerProfiles`))
    (`/Game/MosaicWars/Core/Menu/BP_MenuController.Client_UpdatePlayerReady` _array_element (`self.bIsPlayerReady`))))

(event `self.K2_OnLogout`
  (params (ExitingController :type "Controller Object Reference"))
  ;[1 1 1] Update Player Info on Logout
  (bind _asbp_menu_controller (cast `/Game/MosaicWars/Core/Menu/BP_MenuController` ExitingController))
  (bind _returnvalue (`KismetArrayLibrary.Array_Find` (`self.ConnectedPlayers`) _asbp_menu_controller))
  (`KismetArrayLibrary.Array_Remove` (`self.bIsPlayerReady`) _returnvalue)
  (`KismetArrayLibrary.Array_Remove` (`self.ConnectedPlayers`) _returnvalue)
  (`self.UpdateLobby`))

(event `SetPlayerReady`
  (params (bIsReady :type Boolean) (PlayerController :type "/Game/MosaicWars/Core/Menu/BP_MenuController Object Reference"))
  ;[1 1 1] Toggle player readiness
  (`KismetArrayLibrary.Array_Set` (`self.bIsPlayerReady`) (`KismetArrayLibrary.Array_Find` (`self.ConnectedPlayers`) PlayerController) bIsReady)
  (`self.UpdateLobby`))

(fn `UserConstructionScript`)