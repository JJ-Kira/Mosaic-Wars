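; Player controller for MosaicWars that sets up local input and the game HUD and handles leaving a client session.
; On BeginPlay, the local controller adds the game mapping context, clears widgets, shows a lazily created HUD and switches to game-only input.
; EndClientSession clears the multiplayer pause-menu flag on the GameInstance, destroys the session and opens MainMenu.
; The Interact input handler is empty, with its message call left unconnected.
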(event `self.ReceiveBeginPlay`
  (if (`self.IsLocalPlayerController`)
    (`EnhancedInputSubsystemInterface.AddMappingContext` (subsystem `EnhancedInputLocalPlayerSubsystem`) "/Game/MosaicWars/Core/Input/IMC_Game.IMC_Game" 0 (struct))
    (`WidgetLayoutLibrary.RemoveAllWidgets`)
    (`self.UI_ShowGameHUD`)
    (`WidgetBlueprintLibrary.SetInputMode_GameOnly` self)
    (set `self.bShowMouseCursor` false)))

(event `EnhancedInput|/Game/MosaicWars/Core/Input/Actions/IA_Interact`
  (params (ActionValue :type Boolean) (ElapsedSeconds :type "Float (double-precision)") (TriggeredSeconds :type "Float (double-precision)") (InputAction :type "InputAction Object Reference" :default "/Game/MosaicWars/Core/Input/Actions/IA_Interact.IA_Interact"))
  ;[1 1 1] Trigger interaction
)

(event `ShowGameHUD`
  (`Widget.SetVisibility` (`self.GameHUD`) "Visible"))

(event `EndClientSession`
  (bind _asbp_mosaic_wars_game_instance (cast `/Game/MosaicWars/Core/Multiplayer/BP_MosaicWars_GameInstance` (`GameplayStatics.GetGameInstance`)))
  (set `/Game/MosaicWars/Core/Multiplayer/BP_MosaicWars_GameInstance.bIsPauseMenuVisibleMultiplayer` false _asbp_mosaic_wars_game_instance)
  (`DestroySessionCallbackProxy.DestroySession` self
    (:`then`
      (`GameplayStatics.OpenLevel` "MainMenu"))))

(fn `UI_ShowGameHUD`
  (`/Engine/EditorBlueprintResources/StandardMacros.IsValid` (`self.GameHUD`)
    (:`Is Valid`
      _)
    (:`Is Not Valid`
      (bind _returnvalue (`|CreateWidget` "/Game/MosaicWars/Widgets/WB_GameHUD.WB_GameHUD_C" self))
      (set `self.GameHUD` _returnvalue)))
  (`UserWidget.AddToViewport` (`self.GameHUD`) 0))

(fn `UserConstructionScript`)