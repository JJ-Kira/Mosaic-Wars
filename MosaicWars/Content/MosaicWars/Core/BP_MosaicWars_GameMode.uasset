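; Mosaic Wars game mode that gives each connecting player a platform and a possessed third-person character.
; It gathers player controllers until they match the game instance's player count, then after a short delay spawns and assigns both actors.
; GetSpawnLocation scales corner offsets by the Difficulty value as platform size.
; Its later branches compare constants instead of PlayerIndex, so every player after the first gets the same negative-X, negative-Y corner.
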(event `self.HandleStartingNewPlayer`
  (params (NewPlayer :type "PlayerController Object Reference"))
  (bind _asbp_player_controller (cast `/Game/MosaicWars/Core/BP_PlayerController` NewPlayer))
  (`KismetArrayLibrary.Array_Add` (`self.ConnectedControllers`) _asbp_player_controller)
  (bind _asbp_mosaic_wars_game_instance (cast `/Game/MosaicWars/Core/Multiplayer/BP_MosaicWars_GameInstance` (`GameplayStatics.GetGameInstance`)))
  (bind _output_get (set `self.Number Of Connected Players` (`/Game/MosaicWars/Core/Multiplayer/BP_MosaicWars_GameInstance.NumberOfConnectedPlayers` _asbp_mosaic_wars_game_instance)))
  (if (== _output_get (`KismetArrayLibrary.Array_Length` (`self.ConnectedControllers`)))
    (`KismetSystemLibrary.Delay` 0.5)
    (for (_array_element _array_index) (`self.ConnectedControllers`)
      (bind _spawnlocation (`self.GetSpawnLocation` _array_index (`/Game/MosaicWars/Core/Multiplayer/BP_MosaicWars_GameInstance.Difficulty` _asbp_mosaic_wars_game_instance)))
      (bind _returnvalue (`|SpawnActorFromClass` "/Game/MosaicWars/Game/BP_Platform.BP_Platform_C" (`KismetMathLibrary.MakeTransform` (`KismetMathLibrary.MakeVector` (.x _spawnlocation) (.y _spawnlocation) -50.0)) "Undefined" "MultiplyWithRoot" null null))
      (`self.SetOwner` _returnvalue _array_element)
      (bind _returnvalue_2 (`|SpawnActorFromClass` "/Game/MosaicWars/Core/BP_ThirdPersonCharacter.BP_ThirdPersonCharacter_C" (`KismetMathLibrary.MakeTransform` (`KismetMathLibrary.MakeVector` (.x _spawnlocation) (.y _spawnlocation) 150.0)) "Undefined" "MultiplyWithRoot" null null))
      (`Controller.Possess` _array_element _returnvalue_2))))

(fn `GetSpawnLocation`
  (params (PlayerIndex :type Integer) (PlatformSize :type Integer))
  (returns (SpawnLocation :type "Vector Structure"))
  (bind _returnvalue (+ (* PlatformSize 50) 250))
  (bind _returnvalue_2 (`KismetMathLibrary.Conv_IntToDouble` _returnvalue))
  (bind _returnvalue_3 (`KismetMathLibrary.Conv_IntToDouble` (* _returnvalue -1)))
  (if (== PlayerIndex 0)
    (return (`KismetMathLibrary.MakeVector` _returnvalue_2 _returnvalue_2))
    (elif (== 0 1)
      (return (`KismetMathLibrary.MakeVector` _returnvalue_2 _returnvalue_3))
      (elif (== 0 2)
        (return (`KismetMathLibrary.MakeVector` _returnvalue_3 _returnvalue_2))
        (else
          (return (`KismetMathLibrary.MakeVector` _returnvalue_3 _returnvalue_3)))))))

(fn `UserConstructionScript`)