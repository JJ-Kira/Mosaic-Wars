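; BP_MainMenu_GameMode is the MosaicWars main menu game mode that registers players joining the Lobby level and keeps their lobby player lists in sync.
; When a new player starts on Lobby, it stores their BP_MenuController, has it create the lobby menu and runs its initial setup.
; UpdateLobby, gated by its PlayerNames input, rebuilds the profile list from connected controllers and pushes it back to each one.
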(event `self.HandleStartingNewPlayer`
  (params (NewPlayer :type "PlayerController Object Reference"))
  (bind _returnvalue (`GameplayStatics.GetCurrentLevelName` true))
  (switch `string` _returnvalue
    (:`Lobby`
      (bind _asbp_menu_controller (cast `/Game/MosaicWars/Core/Menu/BP_MenuController` NewPlayer))
      (`KismetArrayLibrary.Array_Add` (`self.ConnectedPlayers`) _asbp_menu_controller)
      (`/Game/MosaicWars/Core/Menu/BP_MenuController.CreateLobbyMenu` _asbp_menu_controller)
      (`/Game/MosaicWars/Core/Menu/BP_MenuController.InitialSetup` _asbp_menu_controller))))

(event `UpdateLobby`
  (params (PlayerNames :type Boolean))
  (if PlayerNames
    (`KismetArrayLibrary.Array_Clear` (`self.PlayerProfiles`))
    (for _array_element (`self.ConnectedPlayers`)
      (`KismetArrayLibrary.Array_Add` (`self.PlayerProfiles`) (`/Game/MosaicWars/Core/Menu/BP_MenuController.LocalPlayerProfile` _array_element)))
    (for _array_element_2 (`self.ConnectedPlayers`)
      (`/Game/MosaicWars/Core/Menu/BP_MenuController.UpdatePlayerNames` _array_element_2 (`self.PlayerProfiles`)))))

(fn `UserConstructionScript`)